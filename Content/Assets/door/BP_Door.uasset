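; Sliding double door that also cues Biju NPC voice-over when its trigger box is overlapped.
; OpenDoor runs two timelines that slide the left and right panels apart along local X.
; If DoorOpen is set, overlap plays the coins-to-invest script through Biju's PlayingScript, provided that audio is valid and idle.
; Reference-getter functions are empty stubs except GetDoorRef, which returns this door.
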(event `self.Box.OnComponentBeginOverlap`
  (params (OverlappedComponent :type "PrimitiveComponent Object Reference") (OtherActor :type "Actor Object Reference") (OtherComp :type "PrimitiveComponent Object Reference") (OtherBodyIndex :type Integer) (bFromSweep :type Boolean) (SweepResult :type "HitResult Structure (by ref)"))
  (if (`self.doorOpen`)
    (bind _returnvalue (`GameplayStatics.GetActorOfClass` "/Game/ThirdPerson/Blueprints/BP_BijuNPC.BP_BijuNPC_C"))
    (bind _bijuref (message `/Game/Blueprint/Interfaces/BP_Interact_Interface.getBijuRef` _returnvalue))
    (bind _playingscript (`/Game/ThirdPerson/Blueprints/BP_BijuNPC.playingScript` _bijuref))
    (if (`KismetSystemLibrary.IsValid` _playingscript)
      (if (not (`AudioComponent.IsPlaying` _playingscript))
        (bind _returnvalue_2 (`GameplayStatics.CreateSound2D` "/Game/Sounds/UPDATE_2/update_bijuScript_coinsToInvest.update_bijuScript_coinsToInvest" 1.0 1.0 0.0 null))
        (bind _output_get (set `/Game/ThirdPerson/Blueprints/BP_BijuNPC.playingScript` _returnvalue_2 _bijuref))
        (`AudioComponent.Play` _output_get 0.0)))))

(event `OpenDoor`
  (`|ExecutionSequence`
    (:`then_0`
      (bind (_direction _rightdoorfloat) (`Timeline|OpenRightDoorTimeline` :!via `PlayFromStart`)
        (:`Update`
          (`SceneComponent.K2_SetRelativeLocation` (`self.door_right`) (`KismetMathLibrary.MakeVector` (`KismetMathLibrary.Lerp` 0.0 1500.0 _rightdoorfloat)) false false))))
    (:`then_1`
      (bind (_direction_2 _leftdooropen) (`Timeline|OpenLeftDoorTimeline` :!via `PlayFromStart`)
        (:`Update`
          (`SceneComponent.K2_SetRelativeLocation` (`self.door_left`) (`KismetMathLibrary.MakeVector` (`KismetMathLibrary.Lerp` 0.0 -1500.0 _leftdooropen)) false false))))))

(fn `getBarRef`
  (returns (barRef :type "/Game/Blueprint/LeaderLounge/BP_Dynamic_bar Object Reference"))
  (return null))

(fn `getBarRefVal`
  (returns (getBarRefVal :type "/Game/Blueprint/LeaderLounge/BP_Dynamic_Value Object Reference"))
  (return null))

(fn `getBijuRef`
  (returns (bijuRef :type "/Game/ThirdPerson/Blueprints/BP_BijuNPC Object Reference"))
  (return null))

(fn `getCircleGraphRef`
  (returns (circleGraphRef :type "/Game/Blueprint/LeaderLounge/BP_CircleGraph Object Reference"))
  (return null))

(fn `getDataLayerRef`
  (returns (dataLayerRef :type "/Game/Blueprint/BP_DataLayer Object Reference"))
  (return null))

(fn `getDoorRef`
  (returns (doorRef :type "/Game/Assets/door/BP_Door Object Reference"))
  (return self))

(fn `getHUDRef`
  (returns (hudRef :type "/Game/RPMCharacterTool/HUD/BP_HUD Object Reference"))
  (return null))

(fn `getRankingRef`
  (returns (rankingRef :type "/Game/Blueprint/LeaderLounge/BP_ranking Object Reference"))
  (return null))

(fn `getTopBrandRef`
  (returns (topBrandRef :type "/Game/Blueprint/BP_LeaderOfWeek Object Reference"))
  (return null))

(fn `getValueBarRef`
  (returns (valueBarref :type "/Game/Blueprint/LeaderLounge/BP_Dynamic_Value Object Reference"))
  (return null))

(fn `UserConstructionScript`)