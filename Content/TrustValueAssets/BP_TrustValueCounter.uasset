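; World display that shows a trust value as ten full or empty meshes plus a 3D text number.
; The construction script gathers the meshes, lays them out in two rows along X and Z, and applies configurable scales and text placement.
; UpdateTrustValue converts the value to five-point steps, fills that many meshes, empties the rest and writes the stepped value to the text.
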(fn `MakeArray`
  (bind _meshes (`self.Meshes`))
  (`KismetArrayLibrary.Array_Add` _meshes (`self.StaticMesh1`))
  (`KismetArrayLibrary.Array_Add` _meshes (`self.StaticMesh2`))
  (`KismetArrayLibrary.Array_Add` _meshes (`self.StaticMesh3`))
  (`KismetArrayLibrary.Array_Add` _meshes (`self.StaticMesh4`))
  (`KismetArrayLibrary.Array_Add` _meshes (`self.StaticMesh`))
  (`KismetArrayLibrary.Array_Add` _meshes (`self.StaticMesh6`))
  (`KismetArrayLibrary.Array_Add` _meshes (`self.StaticMesh7`))
  (`KismetArrayLibrary.Array_Add` _meshes (`self.StaticMesh8`))
  (`KismetArrayLibrary.Array_Add` _meshes (`self.StaticMesh9`))
  (`KismetArrayLibrary.Array_Add` _meshes (`self.StaticMesh5`)))

(fn `SetMeshLocations`
  (params (Integer :type Integer))
  (bind _returnvalue (/ (`KismetArrayLibrary.Array_Length` (`self.Meshes`)) 2))
  (if (< Integer _returnvalue)
    (`SceneComponent.K2_SetRelativeLocation` (`|GetArrayItem` (`self.Meshes`) Integer) (`KismetMathLibrary.MakeVector` (* Integer (`self.X-Distance`))) false false)
    (else
      (`SceneComponent.K2_SetRelativeLocation` (`|GetArrayItem` (`self.Meshes`) Integer) (`KismetMathLibrary.MakeVector` (* (- Integer _returnvalue) (`self.X-Distance`)) 0.0 (`self.Y-Distance`)) false false))))

(fn `UpdateTrustValue`
  (params (TrustValue :type Integer))
  (locals (CurrentTrustValue :type Integer))
  (bind _output_get (set `local.CurrentTrustValue` (/ TrustValue 5)))
  (`Text3DComponent.SetText` (`self.Text3D`) (`KismetTextLibrary.Conv_IntToText` (* _output_get 5)))
  (for (_array_element _array_index) (`self.Meshes`)
    (if (<= _array_index (- (`local.CurrentTrustValue`) 1))
      (`StaticMeshComponent.SetStaticMesh` _array_element (`self.MeshFull`))
      (else
        (`StaticMeshComponent.SetStaticMesh` _array_element (`self.MeshEmpty`))))))

(fn `UserConstructionScript`
  (bind _text3d (`self.Text3D`))
  (`|ExecutionSequence`
    (:`then_0`
      (`self.MakeArray`)
      ;[1 1 1] Set static Mesh Locations
      (for (_array_element _array_index) (`self.Meshes`)
        (`self.SetMeshLocations` _array_index)
        (`StaticMeshComponent.SetStaticMesh` _array_element (`self.MeshFull`))
        (`SceneComponent.SetWorldScale3D` _array_element (* (`SceneComponent.RelativeScale3D` _array_element) (`self.MeshScale`)))))
    (:`then_1`
      (`SceneComponent.K2_SetRelativeLocation` (`self.Text3D`) (`self.TextLocation`) false false)
      (`SceneComponent.SetWorldScale3D` _text3d (* (`SceneComponent.RelativeScale3D` _text3d) (`self.TextScale`))))))