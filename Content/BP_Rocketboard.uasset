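; BP_Rocketboard is an actor that plays a timed intro, then rides a spline path and destroys itself at the end.
; BeginPlay chains delays with two sounds, tells the player character to show the score, finds BP_InitialPathSpline and starts the movement.
; A timeline, rate-scaled by InitialFlowTime, lerps distance along the spline to set location and rotation.
; Score and reference getter functions are empty stubs.
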(event `self.ReceiveBeginPlay`
  (`KismetSystemLibrary.Delay` 2.0)
  (`GameplayStatics.PlaySoundAtLocation` "/Game/Sounds/1.1" (0.0 0.0 0.0) (struct) 1.0 1.0 0.0 null null null null)
  (`KismetSystemLibrary.Delay` 12.0)
  (`GameplayStatics.PlaySoundAtLocation` "/Game/Sounds/2.2" (0.0 0.0 0.0) (struct) 1.0 1.0 0.0 null null null null)
  (`KismetSystemLibrary.Delay` 10.0)
  (bind _player (message `/Game/ThirdPerson/Blueprints/BI_Interaction.GetThirdPersonRef` (`GameplayStatics.GetPlayerCharacter` 0)))
  (`/Game/ThirdPerson/Blueprints/BP_ThirdPersonCharacter.showScore` _player)
  (bind _returnvalue (`GameplayStatics.GetActorOfClass` "/Game/BP_InitialPathSpline.BP_InitialPathSpline_C"))
  (set `self.InitialSplineREF` _returnvalue)
  (`self.MoveRocketBoard`))

(event `MoveRocketBoard`
  (bind _spline (`/Game/BP_InitialPathSpline.Spline` (`self.InitialSplineREF`)))
  (`TimelineComponent.SetPlayRate` (`self.Rocketboard Move T`) (/ 1.0 (`self.InitialFlowTime`)))
  (bind (_direction _move_track) (`Timeline|Rocketboard Move T`)
    (:`Update`
      (bind _returnvalue (`KismetMathLibrary.Lerp` 0.0 (`SplineComponent.GetSplineLength` (`/Game/BP_InitialPathSpline.Spline` (`self.InitialSplineREF`))) _move_track))
      (`self.K2_SetActorTransform` (`KismetMathLibrary.MakeTransform` (`SplineComponent.GetLocationAtDistanceAlongSpline` _spline _returnvalue "World") (`SplineComponent.GetRotationAtDistanceAlongSpline` _spline _returnvalue "Local"))))
    (:`Finished`
      (`self.K2_DestroyActor`))))

(fn `GetInteractionWidgetRef`
  (returns (Ref :type "WidgetComponent Object Reference"))
  (return null))

(fn `getScore`
  (returns (TrustCoins :type Integer) (ValueCoins :type Integer))
  (return 0 0))

(fn `GetThirdPersonRef`
  (returns (Player :type "/Game/ThirdPerson/Blueprints/BP_ThirdPersonCharacter Object Reference"))
  (return null))

(fn `trustSelectedCountRef`
  (returns (CounterTrust :type "/Game/Blueprint/BP_Counter_Trust Object Reference"))
  (return null))

(fn `UserConstructionScript`)

(fn `valueSelectedCountRef`
  (returns (counterValue :type "/Game/Blueprint/BP_Counter_Value Object Reference"))
  (return null))