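; BP_BrandCoin is a brand coin Blueprint with almost no logic of its own.
; Its event graph and construction script are empty, and it exposes getters for itself, the interaction widget, the third-person reference, trust and value selected counts, and score.
; Only the self getter returns a real reference; the score getter returns zero trust and value coins, and the other getters are empty stubs.
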(fn `getBrandCoinRef`
  (returns (getBrandCoinRef :type "/Game/Blueprint/brandCoins/BP_BrandCoin Object Reference"))
  (return self))

(fn `GetInteractionWidgetRef`
  (returns (Ref :type "WidgetComponent Object Reference"))
  (return null))

(fn `getScore`
  (returns (TrustCoins :type Integer) (ValueCoins :type Integer))
  (return 0 0))

(fn `GetThirdPersonRef`
  (returns (Player :type "/Game/ThirdPerson/Blueprints/BP_ThirdPersonCharacter Object Reference"))
  (return null))

(fn `trustSelectedCountRef`
  (returns (CounterTrust :type "/Game/Blueprint/BP_Counter_Trust Object Reference"))
  (return null))

(fn `UserConstructionScript`)

(fn `valueSelectedCountRef`
  (returns (counterValue :type "/Game/Blueprint/BP_Counter_Value Object Reference"))
  (return null))