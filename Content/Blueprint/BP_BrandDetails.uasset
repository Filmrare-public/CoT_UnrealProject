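; BP_BrandDetails is an actor that displays details for a selected brand by swapping the material on its plane geometry.
; The UpdateBrandDetails event uses the selected brand as an index into the Materials array and applies that material to slot 0.
; The reference getters for bars, graphs, HUD, door and other objects are empty stubs, and the construction script does nothing.
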(event `/Game/Blueprint/Interfaces/BP_Interact_Interface.updateBrandDetails`
  (params (selectedbrand :type Integer))
  (`PrimitiveComponent.SetMaterial` (`self.Plane`) 0 (`|GetArrayItem` (`self.materials`) selectedbrand))
  (`PrimitiveComponent.SetMaterial` (`self.Plane`) 0 (`|GetArrayItem` (`self.materials`) selectedbrand)))

(fn `getBarRef`
  (returns (barRef :type "/Game/Blueprint/LeaderLounge/BP_Dynamic_bar Object Reference"))
  (return null))

(fn `getBarRefVal`
  (returns (getBarRefVal :type "/Game/Blueprint/LeaderLounge/BP_Dynamic_Value Object Reference"))
  (return null))

(fn `getBijuRef`
  (returns (bijuRef :type "/Game/ThirdPerson/Blueprints/BP_BijuNPC Object Reference"))
  (return null))

(fn `getCircleGraphRef`
  (returns (circleGraphRef :type "/Game/Blueprint/LeaderLounge/BP_CircleGraph Object Reference"))
  (return null))

(fn `getDataLayerRef`
  (returns (dataLayerRef :type "/Game/Blueprint/BP_DataLayer Object Reference"))
  (return null))

(fn `getDoorRef`
  (returns (doorRef :type "/Game/Assets/door/BP_Door Object Reference"))
  (return null))

(fn `getHUDRef`
  (returns (hudRef :type "/Game/RPMCharacterTool/HUD/BP_HUD Object Reference"))
  (return null))

(fn `getRankingRef`
  (returns (rankingRef :type "/Game/Blueprint/LeaderLounge/BP_ranking Object Reference"))
  (return null))

(fn `getTopBrandRef`
  (returns (topBrandRef :type "/Game/Blueprint/BP_LeaderOfWeek Object Reference"))
  (return null))

(fn `getValueBarRef`
  (returns (valueBarref :type "/Game/Blueprint/LeaderLounge/BP_Dynamic_Value Object Reference"))
  (return null))

(fn `UserConstructionScript`)