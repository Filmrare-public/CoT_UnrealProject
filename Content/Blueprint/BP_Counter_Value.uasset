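; BP_Counter_Value is a counter that displays its SelectedCount as 3D text, apparently for a value selection.
; Tick converts the count to text and pushes it to Text3D every frame; nothing in these graphs changes the count.
; ValueSelectedCountRef returns the counter itself so other objects can reach it.
; The other getters, which look like a shared interface, are stubs returning empty references or zero scores.
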(event `self.ReceiveTick`
  (params (DeltaSeconds :type "Float (single-precision)"))
  (`Text3DComponent.SetText` (`self.Text3D`) (`KismetTextLibrary.Conv_IntToText` (`self.selectedCount`))))

(fn `GetInteractionWidgetRef`
  (returns (Ref :type "WidgetComponent Object Reference"))
  (return null))

(fn `getScore`
  (returns (TrustCoins :type Integer) (ValueCoins :type Integer))
  (return 0 0))

(fn `GetThirdPersonRef`
  (returns (Player :type "/Game/ThirdPerson/Blueprints/BP_ThirdPersonCharacter Object Reference"))
  (return null))

(fn `trustSelectedCountRef`
  (returns (CounterTrust :type "/Game/Blueprint/BP_Counter_Trust Object Reference"))
  (return null))

(fn `UserConstructionScript`)

(fn `valueSelectedCountRef`
  (returns (counterValue :type "/Game/Blueprint/BP_Counter_Value Object Reference"))
  (return self))