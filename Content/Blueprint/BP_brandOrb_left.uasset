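; Interactable left orb that steps the BP_Carousel back to its previous item.
; On BeginPlay it caches the carousel; interaction calls InteractOnServer, which flips InteractToggle, plays a click sound and calls PreviousItem.
; Focus toggles custom depth on InvestTrust for highlighting.
; The InteractToggle OnRep does nothing, and most getter functions are empty stubs, apart from the interaction widget getter.
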(event `self.ReceiveBeginPlay`
  (bind _returnvalue (`GameplayStatics.GetActorOfClass` "/Game/3DCarousel/Blueprint/BP_Carousel.BP_Carousel_C"))
  (set `self.CarouselRef` _returnvalue))

(event `/Game/ThirdPerson/Blueprints/BI_Interaction.InterfaceInteract`
  (`self.InteractOnServer`))

(event `InteractOnServer`
  (set `self.InteractToggle` (not (`self.InteractToggle`)))
  (`GameplayStatics.PlaySoundAtLocation` "/Engine/VREditor/Sounds/UI/Click_on_Button.Click_on_Button" (`self.K2_GetActorLocation`) (struct) 1.0 1.0 0.0 null null null null)
  (`/Game/3DCarousel/Blueprint/BP_Carousel.PreviousItem` (`self.CarouselRef`)))

(event `/Game/ThirdPerson/Blueprints/BI_Interaction.Interface_ToggleFocus`
  (params (Focus :type Boolean))
  (`PrimitiveComponent.SetRenderCustomDepth` (`self.InvestTrust`) Focus))

(fn `getBarRef`
  (returns (barRef :type "/Game/Blueprint/LeaderLounge/BP_Dynamic_bar Object Reference"))
  (return null))

(fn `getBarRefVal`
  (returns (getBarRefVal :type "/Game/Blueprint/LeaderLounge/BP_Dynamic_Value Object Reference"))
  (return null))

(fn `getBijuRef`
  (returns (bijuRef :type "/Game/ThirdPerson/Blueprints/BP_BijuNPC Object Reference"))
  (return null))

(fn `getCircleGraphRef`
  (returns (circleGraphRef :type "/Game/Blueprint/LeaderLounge/BP_CircleGraph Object Reference"))
  (return null))

(fn `getDataLayerRef`
  (returns (dataLayerRef :type "/Game/Blueprint/BP_DataLayer Object Reference"))
  (return null))

(fn `getDoorRef`
  (returns (doorRef :type "/Game/Assets/door/BP_Door Object Reference"))
  (return null))

(fn `getHUDRef`
  (returns (hudRef :type "/Game/RPMCharacterTool/HUD/BP_HUD Object Reference"))
  (return null))

(fn `GetInteractionWidgetRef`
  (returns (Ref :type "WidgetComponent Object Reference"))
  (return (`self.Widget`)))

(fn `getRankingRef`
  (returns (rankingRef :type "/Game/Blueprint/LeaderLounge/BP_ranking Object Reference"))
  (return null))

(fn `getScore`
  (returns (TrustCoins :type Integer) (ValueCoins :type Integer))
  (return 0 0))

(fn `getTopBrandRef`
  (returns (topBrandRef :type "/Game/Blueprint/BP_LeaderOfWeek Object Reference"))
  (return null))

(fn `getValueBarRef`
  (returns (valueBarref :type "/Game/Blueprint/LeaderLounge/BP_Dynamic_Value Object Reference"))
  (return null))

(fn `GetVrPawnRef`
  (returns (Player :type "/Game/VRTemplate/Blueprints/VRPawn Object Reference"))
  (return null))

(fn `InteractEWidgetRef`
  (returns (InteractEwidgetRef :type "/Game/Widgets/WB_pressEbutton Object Reference"))
  (return null))

(fn `OnRep_InteractToggle`
  (if (`self.InteractToggle`)
    _))

(fn `rocketBoardRef`
  (returns (RocketBoardRef :type "/Game/BP_Rocketboard Object Reference"))
  (return null))

(fn `ScoreRef`
  (params (UpdateTrustScore :type Integer) (UpdateValueScore :type Integer))
  (return))

(fn `trustSelectedCountRef`
  (returns (CounterTrust :type "/Game/Blueprint/BP_Counter_Trust Object Reference"))
  (return null))

(fn `UserConstructionScript`)

(fn `valueSelectedCountRef`
  (returns (counterValue :type "/Game/Blueprint/BP_Counter_Value Object Reference"))
  (return null))