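; Data layer Blueprint that loads brand trust and value scores from a Firebase collection and drives the brand ranking displays.
; On BeginPlay it queries brands by descending trust, skips hidden ones, caches scores and takes the first Unilever brand as top.
; After delays it updates BP_ranking bars, BP_CircleGraph coins and BP_LeaderOfWeek.
; UpdateData writes the selected brand's scores back; older data-path fetch, update and manual sort chains are disconnected.
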(event `self.ReceiveBeginPlay`
  (`self.GetTrustData`))

(event `receivedTrustData`
  (bind _trustscorearray (`self.trustScoreArray`))
  (bind _valuescorearray (`self.valueScoreArray`))
  (set `self.trustMax` (`.MaxValue` (`KismetMathLibrary.MaxOfIntArray` _trustscorearray)))
  (set `self.trustMin` (`.MinValue` (`KismetMathLibrary.MinOfIntArray` _trustscorearray)))
  (set `self.valueMax` (`.MaxValue` (`KismetMathLibrary.MaxOfIntArray` _valuescorearray)))
  (set `self.valueMin` (`.MinValue` (`KismetMathLibrary.MinOfIntArray` _valuescorearray)))
  (`KismetSystemLibrary.Delay` 5.0)
  (bind _returnvalue (`GameplayStatics.GetActorOfClass` "/Game/Blueprint/LeaderLounge/BP_ranking.BP_ranking_C"))
  (`/Game/Blueprint/LeaderLounge/BP_ranking.updateBars` _returnvalue)
  (bind _returnvalue_2 (`GameplayStatics.GetActorOfClass` "/Game/Blueprint/LeaderLounge/BP_CircleGraph.BP_CircleGraph_C"))
  (`/Game/Blueprint/LeaderLounge/BP_CircleGraph.addCoins` _returnvalue_2)
  (`KismetSystemLibrary.Delay` 5.0)
  (bind _returnvalue_3 (`GameplayStatics.GetActorOfClass` "/Game/Blueprint/BP_LeaderOfWeek.BP_LeaderOfWeek_C"))
  (`Text3DComponent.SetText` (`/Game/Blueprint/BP_LeaderOfWeek.Text3D` _returnvalue_3) (`KismetTextLibrary.Conv_StringToText` (`self.topUnileverBrand`)))
  (`/Game/Blueprint/BP_LeaderOfWeek.AddBrandCoin` _returnvalue_3 (`self.topUnileverBrandId`)))

(event `GetTrustData`
  (bind _returnvalue (`FBPFirestore.FBPBeginGetCollectionQuery`))
  (bind _returnvalue_2 (`FBCollectionQuery.OrderBy` "trust" false _returnvalue))
  (`FBPFirestore.FBPGetCollection` (`|MakeArray` "brands") _returnvalue_2 (delegate `onDocumentReceived`) (delegate `onFail`)))

(event `onFail`
  (params (ErrorMessage :type String))
  (`KismetSystemLibrary.PrintString` ErrorMessage))

(event `onfailed`
  (params (ErrorMessage :type String))
  ;[1 1 1] getTrustScore
  ;;[1 1 1] failed callback
  (`KismetSystemLibrary.PrintString` ErrorMessage))

(event `CustomEvent_1`
  (params (ErrorMessage :type String))
  ;[1 1 1] getValueScore
  ;;[1 1 1] failed callback
  (`KismetSystemLibrary.PrintString` ErrorMessage))

(event `onDocumentReceived`
  (params (CollectionSnapshot :type "CollectionSnapshot Structure"))
  ;[1 1 1] success callback
  (bind _returnvalue (`FBPFirestore.FBPGetDocumentsFromCollection` CollectionSnapshot))
  (set `self.topUnileverBrand` "NIL")
  (for _array_element _returnvalue
    (bind _returnvalue_2 (`FBPDataObject.GetString` "id" _array_element))
    (bind _returnvalue_3 (`FBPDataObject.GetNumber` "trust" _array_element))
    (if (not (`BlueprintMapLibrary.Map_Contains` (`self.brandsToHide`) _returnvalue_2))
      (bind _returnvalue_4 (`FBPDataObject.GetNumber` "value" _array_element))
      (`BlueprintMapLibrary.Map_Add` (`self.TrustScore`) _returnvalue_2 (`KismetMathLibrary.FTrunc` _returnvalue_3))
      (`KismetArrayLibrary.Array_Add` (`self.trustScoreArray`) (`KismetMathLibrary.FTrunc` _returnvalue_3))
      (bind _returnvalue_5 (`KismetMathLibrary.FTrunc` _returnvalue_4))
      (`BlueprintMapLibrary.Map_Add` (`self.ValueScore`) _returnvalue_2 _returnvalue_5)
      (`KismetArrayLibrary.Array_Add` (`self.valueScoreArray`) _returnvalue_5)
      (bind _returnvalue_6 (`FBPDataObject.GetBoolean` "unilever" _array_element))
      (if (and _returnvalue_6 (== (`self.topUnileverBrand`) "NIL"))
        (bind _returnvalue_7 (`FBPDataObject.GetString` "name" _array_element))
        (set `self.topUnileverBrand` _returnvalue_7)
        ;[1 1 1] getTrustScore
        (set `self.topUnileverBrandId` _returnvalue_2))))
  (`self.receivedTrustData`))

(event `OnValuereceived`
  (params (DataSnapshot :type "DocumentSnapshot Structure"))
  (bind _temptrustscore (`self.tempTrustScore`))
  ;[1 1 1] getTrustScore
  ;;[1 1 1] success callback
  (bind _keys (`BlueprintMapLibrary.Map_Keys` _temptrustscore))
  (for _array_element _keys
    (bind _returnvalue (`FBPDataObject.GetMap` _array_element DataSnapshot))
    (`|ExecutionSequence`
      (:`then_0`
        (`FBPDataObject.GetString` "name" _returnvalue))
      (:`then_1`
        (bind _returnvalue_2 (`FBPDataObject.GetNumber` "trust" _returnvalue))
        (bind _returnvalue_3 (`KismetMathLibrary.FTrunc` _returnvalue_2))
        (`BlueprintMapLibrary.Map_Add` _temptrustscore _array_element _returnvalue_3)
        (`KismetArrayLibrary.Array_Add` (`self.tempTrustScoreArray`) _returnvalue_3)))))

(event `CustomEvent`
  (params (DataSnapshot :type "DocumentSnapshot Structure"))
  (bind _tempvaluescore (`self.tempValueScore`))
  ;[1 1 1] getValueScore
  ;;[1 1 1] success callback
  (bind _keys (`BlueprintMapLibrary.Map_Keys` _tempvaluescore))
  (for _array_element _keys
    (bind _returnvalue (`FBPDataObject.GetMap` _array_element DataSnapshot))
    (`|ExecutionSequence`
      (:`then_0`
        (`FBPDataObject.GetString` "name" _returnvalue))
      (:`then_1`
        (bind _returnvalue_2 (`FBPDataObject.GetNumber` "value" _returnvalue))
        (bind _returnvalue_3 (`KismetMathLibrary.FTrunc` _returnvalue_2))
        (`BlueprintMapLibrary.Map_Add` _tempvaluescore _array_element _returnvalue_3)
        (`KismetArrayLibrary.Array_Add` (`self.tempValueScoreArray`) _returnvalue_3)))))

(event `updateFailed`
  (params (ErrorMessage :type String)))

(event `sortTrustScore`)

(event `updateSuccess`
  (params (DataId :type String)))

(event `updateData`
  (bind _selectedbrand (`self.selectedBrand`))
  (bind _returnvalue (`FBPDataObject.FBPBeginWriteDocument`))
  (bind _returnvalue_2 (`FBPDataObject.AddNumber` "trust" (`KismetStringLibrary.Conv_StringToDouble` (`KismetStringLibrary.Conv_IntToString` (`BlueprintMapLibrary.Map_Find` (`self.TrustScore`) _selectedbrand))) _returnvalue))
  (bind _returnvalue_3 (`FBPDataObject.AddNumber` "value" (`KismetStringLibrary.Conv_StringToDouble` (`KismetStringLibrary.Conv_IntToString` (`BlueprintMapLibrary.Map_Find` (`self.ValueScore`) _selectedbrand))) _returnvalue_2))
  (`FBPFirestore.FBPUpdateDocument` (`|MakeArray` "brands" _selectedbrand) _returnvalue_3 (delegate `documentUpdated`) (delegate `documentUpdateFailed`)))

(event `documentUpdated`
  (params (DocumentID :type String)))

(event `documentUpdateFailed`
  (params (ErrorMessage :type String)))

(fn `getBarRef`
  (returns (barRef :type "/Game/Blueprint/LeaderLounge/BP_Dynamic_bar Object Reference"))
  (return null))

(fn `getBarRefVal`
  (returns (getBarRefVal :type "/Game/Blueprint/LeaderLounge/BP_Dynamic_Value Object Reference"))
  (return null))

(fn `getBijuRef`
  (returns (bijuRef :type "/Game/ThirdPerson/Blueprints/BP_BijuNPC Object Reference"))
  (return null))

(fn `getCircleGraphRef`
  (returns (circleGraphRef :type "/Game/Blueprint/LeaderLounge/BP_CircleGraph Object Reference"))
  (return null))

(fn `getDataLayerRef`
  (returns (dataLayerRef :type "/Game/Blueprint/BP_DataLayer Object Reference"))
  (return self))

(fn `getDoorRef`
  (returns (doorRef :type "/Game/Assets/door/BP_Door Object Reference"))
  (return null))

(fn `getHUDRef`
  (returns (hudRef :type "/Game/RPMCharacterTool/HUD/BP_HUD Object Reference"))
  (return null))

(fn `getRankingRef`
  (returns (rankingRef :type "/Game/Blueprint/LeaderLounge/BP_ranking Object Reference"))
  (return null))

(fn `getTopBrandRef`)

(fn `getValueBarRef`
  (returns (valueBarref :type "/Game/Blueprint/LeaderLounge/BP_Dynamic_Value Object Reference"))
  (return null))

(fn `UserConstructionScript`)