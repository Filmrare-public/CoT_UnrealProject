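; BP_InteractableObject is an interactable actor that highlights on focus and plays a click sound when used.
; Interface events drive custom depth on its static mesh and call InteractOnServer, which flips InteractToggle and plays the sound at the actor's location.
; BeginPlay caches in/out mesh transforms and enables input, but nothing here uses those transforms and OnRep_InteractToggle is empty.
; It returns its interaction widget, while score and character getters are stubs.
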(event `self.ReceiveBeginPlay`
  (bind (_returnvalue_location _returnvalue_rotation _returnvalue_scale) (`KismetMathLibrary.BreakTransform` (`SceneComponent.GetRelativeTransform` (`self.StaticMesh`))))
  (set `self.outPosition` (`KismetMathLibrary.MakeTransform` _returnvalue_location _returnvalue_rotation _returnvalue_scale))
  (set `self.inPosition` (`KismetMathLibrary.MakeTransform` (+ _returnvalue_location (0.0 10.0 0.0)) _returnvalue_rotation _returnvalue_scale))
  (`self.EnableInput` (`GameplayStatics.GetPlayerController` 0)))

(event `/Game/ThirdPerson/Blueprints/BI_Interaction.Interface_ToggleFocus`
  (params (Focus :type Boolean))
  (`PrimitiveComponent.SetRenderCustomDepth` (`self.StaticMesh`) Focus))

(event `/Game/ThirdPerson/Blueprints/BI_Interaction.InterfaceInteract`
  (`self.InteractOnServer`))

(event `InteractOnServer`
  (set `self.InteractToggle` (not (`self.InteractToggle`)))
  (`GameplayStatics.PlaySoundAtLocation` "/Engine/VREditor/Sounds/UI/Click_on_Button.Click_on_Button" (`self.K2_GetActorLocation`) (struct) 1.0 1.0 0.0 null null null null))

(fn `GetInteractionWidgetRef`
  (returns (Ref :type "WidgetComponent Object Reference"))
  (return (`self.Widget`)))

(fn `getScore`
  (returns (TrustCoins :type Integer) (ValueCoins :type Integer))
  (return 0 0))

(fn `GetThirdPersonRef`
  (returns (Player :type "/Game/ThirdPerson/Blueprints/BP_ThirdPersonCharacter Object Reference"))
  (return null))

(fn `OnRep_InteractToggle`
  (if (`self.InteractToggle`)
    _))

(fn `ScoreRef`
  (params (UpdateTrustScore :type Integer) (UpdateValueScore :type Integer))
  (return))

(fn `trustSelectedCountRef`
  (returns (CounterTrust :type "/Game/Blueprint/BP_Counter_Trust Object Reference"))
  (return null))

(fn `UserConstructionScript`)

(fn `valueSelectedCountRef`
  (returns (counterValue :type "/Game/Blueprint/BP_Counter_Value Object Reference"))
  (return null))