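; Interactable button that invests the player's selected value coins in the currently selected brand.
; A press plays a click and slides the mesh in and back, then adds the count from BP_Counter_Value to the brand's BP_DataLayer score.
; It deducts the VR pawn's coins, refreshes BP_ValueCounter, and notifies BP_BijuNPC on first investment or when later ones empty the balance.
; Actors communicate through interface reference getters; focus toggles custom-depth highlighting.
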(event `self.ReceiveBeginPlay`
  (bind (_returnvalue_location _returnvalue_rotation _returnvalue_scale) (`KismetMathLibrary.BreakTransform` (`SceneComponent.GetRelativeTransform` (`self.InvestValue`))))
  (set `self.outPosition` (`KismetMathLibrary.MakeTransform` _returnvalue_location _returnvalue_rotation _returnvalue_scale))
  (set `self.inPosition` (`KismetMathLibrary.MakeTransform` (+ _returnvalue_location (0.0 10.0 0.0)) _returnvalue_rotation _returnvalue_scale))
  (`self.EnableInput` (`GameplayStatics.GetPlayerController` 0))
  (bind _outactors (`GameplayStatics.GetAllActorsOfClass` "/Game/TrustValueAssets/BP_ValueCounter.BP_ValueCounter_C"))
  (set `self.ValueCounterReference` (`|GetArrayItem` _outactors)))

(event `/Game/ThirdPerson/Blueprints/BI_Interaction.InterfaceInteract`
  (`self.InteractOnServer`))

(event `InteractOnServer`
  (set `self.InteractToggle` (not (`self.InteractToggle`)))
  (`GameplayStatics.PlaySoundAtLocation` "/Engine/VREditor/Sounds/UI/Click_on_Button.Click_on_Button" (`self.K2_GetActorLocation`) (struct) 1.0 1.0 0.0 null null null null)
  (bind (_direction _buttonin) (`Timeline|ButtonIn` :!via `PlayFromStart`)
    (:`Update`
      (`SceneComponent.K2_SetRelativeTransform` (`self.InvestValue`) (`KismetMathLibrary.TLerp` (`self.outPosition`) (`self.inPosition`) _buttonin) false false))
    (:`Finished`
      (bind (_direction_2 _buttonin_2) (`Timeline|Timeline_0` :!via `ReverseFromEnd`)
        (:`Update`
          (`SceneComponent.K2_SetRelativeTransform` (`self.InvestValue`) (`KismetMathLibrary.TLerp` (`self.outPosition`) (`self.inPosition`) _buttonin_2) false false))
        (:`Finished`
          (`|ExecutionSequence`
            (:`then_0`
              (bind _returnvalue (`GameplayStatics.GetActorOfClass` "/Game/Blueprint/BP_Counter_Value.BP_Counter_Value_C"))
              (bind _countervalue (`/Game/ThirdPerson/Blueprints/BI_Interaction.valueSelectedCountRef` _returnvalue))
              (bind _returnvalue_2 (`GameplayStatics.GetActorOfClass` "/Game/Blueprint/BP_DataLayer.BP_DataLayer_C"))
              (bind _datalayerref (message `/Game/Blueprint/Interfaces/BP_Interact_Interface.getDataLayerRef` _returnvalue_2))
              (bind _valuescore (`/Game/Blueprint/BP_DataLayer.ValueScore` _datalayerref))
              (bind _selectedbrand (`/Game/Blueprint/BP_DataLayer.selectedBrand` _datalayerref))
              (bind _selectedcount (`/Game/Blueprint/BP_Counter_Value.selectedCount` _countervalue))
              (`BlueprintMapLibrary.Map_Add` _valuescore _selectedbrand (+ _selectedcount (`BlueprintMapLibrary.Map_Find` _valuescore _selectedbrand))))
            (:`then_1`
              (bind _player (message `/Game/ThirdPerson/Blueprints/BI_Interaction.GetVrPawnRef` (`GameplayStatics.GetPlayerPawn` 0)))
              (bind _output_get (set `/Game/VRTemplate/Blueprints/VRPawn.ValueCoin` (`KismetMathLibrary.Clamp` (- (`/Game/VRTemplate/Blueprints/VRPawn.ValueCoin` _player) _selectedcount) 0 50) _player))
              (`/Game/TrustValueAssets/BP_TrustValueCounter.UpdateTrustValue` (`self.ValueCounterReference`) _output_get)
              (set `/Game/Blueprint/BP_Counter_Value.selectedCount` 0 _countervalue)
              (if (`self.firstTime`)
                (bind _returnvalue_3 (`GameplayStatics.GetActorOfClass` "/Game/ThirdPerson/Blueprints/BP_BijuNPC.BP_BijuNPC_C"))
                (bind _bijuref (message `/Game/Blueprint/Interfaces/BP_Interact_Interface.getBijuRef` _returnvalue_3))
                (`/Game/ThirdPerson/Blueprints/BP_BijuNPC.ValueInvested` _bijuref)
                (set `self.firstTime` false)
                (elif (<= _output_get 0)
                  (bind _returnvalue_4 (`GameplayStatics.GetActorOfClass` "/Game/ThirdPerson/Blueprints/BP_BijuNPC.BP_BijuNPC_C"))
                  (bind _bijuref_2 (message `/Game/Blueprint/Interfaces/BP_Interact_Interface.getBijuRef` _returnvalue_4))
                  (`/Game/ThirdPerson/Blueprints/BP_BijuNPC.FinishedInvesting` _bijuref_2))))))))))

(event `/Game/ThirdPerson/Blueprints/BI_Interaction.Interface_ToggleFocus`
  (params (Focus :type Boolean))
  (`PrimitiveComponent.SetRenderCustomDepth` (`self.InvestValue`) Focus))

(fn `getBarRef`
  (returns (barRef :type "/Game/Blueprint/LeaderLounge/BP_Dynamic_bar Object Reference"))
  (return null))

(fn `getBarRefVal`
  (returns (getBarRefVal :type "/Game/Blueprint/LeaderLounge/BP_Dynamic_Value Object Reference"))
  (return null))

(fn `getBijuRef`
  (returns (bijuRef :type "/Game/ThirdPerson/Blueprints/BP_BijuNPC Object Reference"))
  (return null))

(fn `getCircleGraphRef`
  (returns (circleGraphRef :type "/Game/Blueprint/LeaderLounge/BP_CircleGraph Object Reference"))
  (return null))

(fn `getDataLayerRef`
  (returns (dataLayerRef :type "/Game/Blueprint/BP_DataLayer Object Reference"))
  (return null))

(fn `getDoorRef`
  (returns (doorRef :type "/Game/Assets/door/BP_Door Object Reference"))
  (return null))

(fn `getHUDRef`
  (returns (hudRef :type "/Game/RPMCharacterTool/HUD/BP_HUD Object Reference"))
  (return null))

(fn `GetInteractionWidgetRef`
  (returns (Ref :type "WidgetComponent Object Reference"))
  (return (`self.Widget`)))

(fn `getRankingRef`
  (returns (rankingRef :type "/Game/Blueprint/LeaderLounge/BP_ranking Object Reference"))
  (return null))

(fn `getScore`
  (returns (TrustCoins :type Integer) (ValueCoins :type Integer))
  (return 0 0))

(fn `getTopBrandRef`
  (returns (topBrandRef :type "/Game/Blueprint/BP_LeaderOfWeek Object Reference"))
  (return null))

(fn `getValueBarRef`
  (returns (valueBarref :type "/Game/Blueprint/LeaderLounge/BP_Dynamic_Value Object Reference"))
  (return null))

(fn `GetVrPawnRef`
  (returns (Player :type "/Game/VRTemplate/Blueprints/VRPawn Object Reference"))
  (return null))

(fn `InteractEWidgetRef`
  (returns (InteractEwidgetRef :type "/Game/Widgets/WB_pressEbutton Object Reference"))
  (return null))

(fn `OnRep_InteractToggle`
  (if (`self.InteractToggle`)
    _))

(fn `rocketBoardRef`
  (returns (RocketBoardRef :type "/Game/BP_Rocketboard Object Reference"))
  (return null))

(fn `ScoreRef`
  (params (UpdateTrustScore :type Integer) (UpdateValueScore :type Integer))
  (return))

(fn `trustSelectedCountRef`
  (returns (CounterTrust :type "/Game/Blueprint/BP_Counter_Trust Object Reference"))
  (return null))

(fn `UserConstructionScript`)

(fn `valueSelectedCountRef`
  (returns (counterValue :type "/Game/Blueprint/BP_Counter_Value Object Reference"))
  (return null))