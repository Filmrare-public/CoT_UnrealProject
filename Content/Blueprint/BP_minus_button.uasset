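; Interactable minus button that lowers the selected trust count on BP_Counter_Trust by 5, clamped between zero and the player pawn's TrustCoin.
; Focus toggles custom depth on the mesh, and interaction calls InteractOnServer, which flips InteractToggle and plays a click sound.
; Two chained timelines lerp the mesh in and back out along local Y, and the count changes only when the return finishes.
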(event `self.ReceiveBeginPlay`
  (bind (_returnvalue_location _returnvalue_rotation _returnvalue_scale) (`KismetMathLibrary.BreakTransform` (`SceneComponent.GetRelativeTransform` (`self.StaticMesh`))))
  (set `self.outPosition` (`KismetMathLibrary.MakeTransform` _returnvalue_location _returnvalue_rotation _returnvalue_scale))
  (set `self.inPosition` (`KismetMathLibrary.MakeTransform` (+ _returnvalue_location (0.0 10.0 0.0)) _returnvalue_rotation _returnvalue_scale)))

(event `/Game/ThirdPerson/Blueprints/BI_Interaction.Interface_ToggleFocus`
  (params (Focus :type Boolean))
  (`PrimitiveComponent.SetRenderCustomDepth` (`self.StaticMesh`) Focus))

(event `/Game/ThirdPerson/Blueprints/BI_Interaction.InterfaceInteract`
  (`self.InteractOnServer`))

(event `InteractOnServer`
  (set `self.InteractToggle` (not (`self.InteractToggle`)))
  (`GameplayStatics.PlaySoundAtLocation` "/Engine/VREditor/Sounds/UI/Click_on_Button.Click_on_Button" (`self.K2_GetActorLocation`) (struct) 1.0 1.0 0.0 null null null null)
  (bind (_direction _buttonin) (`Timeline|Timeline` :!via `PlayFromStart`)
    (:`Update`
      (`SceneComponent.K2_SetRelativeTransform` (`self.StaticMesh`) (`KismetMathLibrary.TLerp` (`self.outPosition`) (`self.inPosition`) _buttonin) false false))
    (:`Finished`
      (bind (_direction_2 _buttonin_2) (`Timeline|Timeline_0` :!via `ReverseFromEnd`)
        (:`Update`
          (`SceneComponent.K2_SetRelativeTransform` (`self.StaticMesh`) (`KismetMathLibrary.TLerp` (`self.outPosition`) (`self.inPosition`) _buttonin_2) false false))
        (:`Finished`
          (bind _returnvalue (`GameplayStatics.GetActorOfClass` "/Game/Blueprint/BP_Counter_Trust.BP_Counter_Trust_C"))
          (bind _countertrust (`/Game/ThirdPerson/Blueprints/BI_Interaction.trustSelectedCountRef` _returnvalue))
          (bind _player (message `/Game/ThirdPerson/Blueprints/BI_Interaction.GetVrPawnRef` (`GameplayStatics.GetPlayerPawn` 0)))
          (set `/Game/Blueprint/BP_Counter_Trust.selectedCount` (`KismetMathLibrary.Clamp` (- (`/Game/Blueprint/BP_Counter_Trust.selectedCount` _countertrust) 5) 0 (`/Game/VRTemplate/Blueprints/VRPawn.TrustCoin` _player)) _countertrust))))))

(fn `getBarRef`
  (returns (barRef :type "/Game/Blueprint/LeaderLounge/BP_Dynamic_bar Object Reference"))
  (return null))

(fn `getBarRefVal`
  (returns (getBarRefVal :type "/Game/Blueprint/LeaderLounge/BP_Dynamic_Value Object Reference"))
  (return null))

(fn `getBijuRef`
  (returns (bijuRef :type "/Game/ThirdPerson/Blueprints/BP_BijuNPC Object Reference"))
  (return null))

(fn `getCircleGraphRef`
  (returns (circleGraphRef :type "/Game/Blueprint/LeaderLounge/BP_CircleGraph Object Reference"))
  (return null))

(fn `getDataLayerRef`
  (returns (dataLayerRef :type "/Game/Blueprint/BP_DataLayer Object Reference"))
  (return null))

(fn `getDoorRef`
  (returns (doorRef :type "/Game/Assets/door/BP_Door Object Reference"))
  (return null))

(fn `getHUDRef`
  (returns (hudRef :type "/Game/RPMCharacterTool/HUD/BP_HUD Object Reference"))
  (return null))

(fn `GetInteractionWidgetRef`
  (returns (Ref :type "WidgetComponent Object Reference"))
  (return (`self.Widget`)))

(fn `getRankingRef`
  (returns (rankingRef :type "/Game/Blueprint/LeaderLounge/BP_ranking Object Reference"))
  (return null))

(fn `getScore`
  (returns (TrustCoins :type Integer) (ValueCoins :type Integer))
  (return 0 0))

(fn `getTopBrandRef`
  (returns (topBrandRef :type "/Game/Blueprint/BP_LeaderOfWeek Object Reference"))
  (return null))

(fn `getValueBarRef`
  (returns (valueBarref :type "/Game/Blueprint/LeaderLounge/BP_Dynamic_Value Object Reference"))
  (return null))

(fn `GetVrPawnRef`
  (returns (Player :type "/Game/VRTemplate/Blueprints/VRPawn Object Reference"))
  (return null))

(fn `InteractEWidgetRef`
  (returns (InteractEwidgetRef :type "/Game/Widgets/WB_pressEbutton Object Reference"))
  (return null))

(fn `OnRep_InteractToggle`
  (if (`self.InteractToggle`)
    _))

(fn `rocketBoardRef`
  (returns (RocketBoardRef :type "/Game/BP_Rocketboard Object Reference"))
  (return null))

(fn `ScoreRef`
  (params (UpdateTrustScore :type Integer) (UpdateValueScore :type Integer))
  (return))

(fn `trustSelectedCountRef`
  (returns (CounterTrust :type "/Game/Blueprint/BP_Counter_Trust Object Reference"))
  (return null))

(fn `UserConstructionScript`)

(fn `valueSelectedCountRef`
  (returns (counterValue :type "/Game/Blueprint/BP_Counter_Value Object Reference"))
  (return null))