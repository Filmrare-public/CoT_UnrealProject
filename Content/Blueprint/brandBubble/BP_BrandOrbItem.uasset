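; Interactable brand orb that lets the player pick a brand on BP_Carousel.
; Interact or mesh touch writes the orb's name to BP_DataLayer as SelectedOrb, then rotates the carousel to it.
; Focus toggles custom depth on the mesh and, until a first brand is selected, pauses carousel rotation, resuming it with NextItem on focus loss.
; References pass through interface getters, mostly empty here except GetOrbRef returning self.
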(event `self.ReceiveBeginPlay`
  (`self.EnableInput` (`GameplayStatics.GetPlayerController` 0))
  (bind _returnvalue (`GameplayStatics.GetActorOfClass` "/Game/3DCarousel/Blueprint/BP_Carousel.BP_Carousel_C"))
  (set `self.carouselRef` _returnvalue))

(event `/Game/ThirdPerson/Blueprints/BI_Interaction.InterfaceInteract`
  (bind _returnvalue (`GameplayStatics.GetActorOfClass` "/Game/Blueprint/BP_DataLayer.BP_DataLayer_C" :!label _label))
  (bind _datalayerref (message `/Game/Blueprint/Interfaces/BP_Interact_Interface.getDataLayerRef` _returnvalue))
  (set `/Game/Blueprint/BP_DataLayer.selectedOrb` (`KismetStringLibrary.Conv_NameToString` (`self.orbName`)) _datalayerref)
  (`/Game/3DCarousel/Blueprint/BP_Carousel.RotateToSelectedOrb` (`self.carouselRef`)))

(event `self.StaticMesh.OnInputTouchBegin`
  (params (FingerIndex :type "ETouchIndex Enum" :default "Touch1") (TouchedComponent :type "PrimitiveComponent Object Reference"))
  (goto _label))

(event `/Game/ThirdPerson/Blueprints/BI_Interaction.Interface_ToggleFocus`
  (params (Focus :type Boolean))
  (`PrimitiveComponent.SetRenderCustomDepth` (`self.StaticMesh`) Focus)
  (bind _returnvalue (`GameplayStatics.GetActorOfClass` "/Game/3DCarousel/Blueprint/BP_Carousel.BP_Carousel_C"))
  (bind _carouselref (message `/Game/Blueprint/brandBubble/BI_BrandOrbInterface.getCarouselRef` _returnvalue))
  (if (not (`/Game/3DCarousel/Blueprint/BP_Carousel.firstBrandSelected` _carouselref))
    (set `/Game/3DCarousel/Blueprint/BP_Carousel.keepRotating` (not Focus) _carouselref)
    (if (not Focus)
      (set `/Game/3DCarousel/Blueprint/BP_Carousel.fromOrbSelection` true _carouselref)
      (set `/Game/3DCarousel/Blueprint/BP_Carousel.resetSelection` false _carouselref)
      (`/Game/3DCarousel/Blueprint/BP_Carousel.NextItem` _carouselref))))

(fn `getBarRef`
  (returns (barRef :type "/Game/Blueprint/LeaderLounge/BP_Dynamic_bar Object Reference"))
  (return null))

(fn `getBarRefVal`
  (returns (getBarRefVal :type "/Game/Blueprint/LeaderLounge/BP_Dynamic_Value Object Reference"))
  (return null))

(fn `getBijuRef`
  (returns (bijuRef :type "/Game/ThirdPerson/Blueprints/BP_BijuNPC Object Reference"))
  (return null))

(fn `getCarouselRef`
  (returns (carouselRef :type "/Game/3DCarousel/Blueprint/BP_Carousel Object Reference"))
  (return null))

(fn `getCircleGraphRef`
  (returns (circleGraphRef :type "/Game/Blueprint/LeaderLounge/BP_CircleGraph Object Reference"))
  (return null))

(fn `getDataLayerRef`
  (returns (dataLayerRef :type "/Game/Blueprint/BP_DataLayer Object Reference"))
  (return null))

(fn `getDoorRef`
  (returns (doorRef :type "/Game/Assets/door/BP_Door Object Reference"))
  (return null))

(fn `getHUDRef`
  (returns (hudRef :type "/Game/RPMCharacterTool/HUD/BP_HUD Object Reference"))
  (return null))

(fn `GetInteractionWidgetRef`
  (returns (Ref :type "WidgetComponent Object Reference"))
  (return null))

(fn `getOrbRef`
  (returns (orbRef :type "/Game/Blueprint/brandBubble/BP_BrandOrbItem Object Reference"))
  (return self))

(fn `getRankingRef`
  (returns (rankingRef :type "/Game/Blueprint/LeaderLounge/BP_ranking Object Reference"))
  (return null))

(fn `getScore`
  (returns (TrustCoins :type Integer) (ValueCoins :type Integer))
  (return 0 0))

(fn `GetThirdPersonRef`
  (returns (Player :type "/Game/ThirdPerson/Blueprints/BP_ThirdPersonCharacter Object Reference"))
  (return null))

(fn `getTopBrandRef`
  (returns (topBrandRef :type "/Game/Blueprint/BP_LeaderOfWeek Object Reference"))
  (return null))

(fn `getValueBarRef`
  (returns (valueBarref :type "/Game/Blueprint/LeaderLounge/BP_Dynamic_Value Object Reference"))
  (return null))

(fn `InteractEWidgetRef`
  (returns (InteractEwidgetRef :type "/Game/Widgets/WB_pressEbutton Object Reference"))
  (return null))

(fn `rocketBoardRef`
  (returns (RocketBoardRef :type "/Game/BP_Rocketboard Object Reference"))
  (return null))

(fn `trustSelectedCountRef`
  (returns (CounterTrust :type "/Game/Blueprint/BP_Counter_Trust Object Reference"))
  (return null))

(fn `UserConstructionScript`)

(fn `valueSelectedCountRef`
  (returns (counterValue :type "/Game/Blueprint/BP_Counter_Value Object Reference"))
  (return null))