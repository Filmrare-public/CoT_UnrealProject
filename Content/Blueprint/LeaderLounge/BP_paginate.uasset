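; BP_paginate is an interactable button in the Leader Lounge that flips the ranking board between its two pages.
; Interaction calls InteractOnServer, which toggles InteractToggle, plays a click, flips the BP_ranking page, refreshes its brand coins and bars, and adds coins on BP_CircleGraph.
; Focus toggles custom depth on the InvestTrust component for highlighting.
; The cached carousel reference is unused, and the OnRep and most interface getters are empty stubs.
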(event `self.ReceiveBeginPlay`
  (bind _returnvalue (`GameplayStatics.GetActorOfClass` "/Game/3DCarousel/Blueprint/BP_Carousel.BP_Carousel_C"))
  (set `self.CarouselRef` _returnvalue))

(event `/Game/ThirdPerson/Blueprints/BI_Interaction.InterfaceInteract`
  (`self.InteractOnServer`))

(event `InteractOnServer`
  (set `self.InteractToggle` (not (`self.InteractToggle`)))
  (`GameplayStatics.PlaySoundAtLocation` "/Engine/VREditor/Sounds/UI/Click_on_Button.Click_on_Button" (`self.K2_GetActorLocation`) (struct) 1.0 1.0 0.0 null null null null)
  (bind _returnvalue (`GameplayStatics.GetActorOfClass` "/Game/Blueprint/LeaderLounge/BP_ranking.BP_ranking_C"))
  (bind _rankingref (message `/Game/Blueprint/Interfaces/BP_Interact_Interface.getRankingRef` _returnvalue))
  (set `/Game/Blueprint/LeaderLounge/BP_ranking.pageNumber` (not (`/Game/Blueprint/LeaderLounge/BP_ranking.pageNumber` _rankingref)) _rankingref)
  (`/Game/Blueprint/LeaderLounge/BP_ranking.addbrandcoins` _rankingref)
  (`/Game/Blueprint/LeaderLounge/BP_ranking.updateBars` _rankingref)
  (bind _returnvalue_2 (`GameplayStatics.GetActorOfClass` "/Game/Blueprint/LeaderLounge/BP_CircleGraph.BP_CircleGraph_C"))
  (bind _circlegraphref (message `/Game/Blueprint/Interfaces/BP_Interact_Interface.getCircleGraphRef` _returnvalue_2))
  (`/Game/Blueprint/LeaderLounge/BP_CircleGraph.addCoins` _circlegraphref))

(event `/Game/ThirdPerson/Blueprints/BI_Interaction.Interface_ToggleFocus`
  (params (Focus :type Boolean))
  (`PrimitiveComponent.SetRenderCustomDepth` (`self.InvestTrust`) Focus))

(fn `getBarRef`
  (returns (barRef :type "/Game/Blueprint/LeaderLounge/BP_Dynamic_bar Object Reference"))
  (return null))

(fn `getBarRefVal`
  (returns (getBarRefVal :type "/Game/Blueprint/LeaderLounge/BP_Dynamic_Value Object Reference"))
  (return null))

(fn `getBijuRef`
  (returns (bijuRef :type "/Game/ThirdPerson/Blueprints/BP_BijuNPC Object Reference"))
  (return null))

(fn `getCircleGraphRef`
  (returns (circleGraphRef :type "/Game/Blueprint/LeaderLounge/BP_CircleGraph Object Reference"))
  (return null))

(fn `getDataLayerRef`
  (returns (dataLayerRef :type "/Game/Blueprint/BP_DataLayer Object Reference"))
  (return null))

(fn `getDoorRef`
  (returns (doorRef :type "/Game/Assets/door/BP_Door Object Reference"))
  (return null))

(fn `GetInteractionWidgetRef`
  (returns (Ref :type "WidgetComponent Object Reference"))
  (return (`self.Widget`)))

(fn `getRankingRef`
  (returns (rankingRef :type "/Game/Blueprint/LeaderLounge/BP_ranking Object Reference"))
  (return null))

(fn `getScore`
  (returns (TrustCoins :type Integer) (ValueCoins :type Integer))
  (return 0 0))

(fn `GetThirdPersonRef`
  (returns (Player :type "/Game/ThirdPerson/Blueprints/BP_ThirdPersonCharacter Object Reference"))
  (return null))

(fn `getValueBarRef`
  (returns (valueBarref :type "/Game/Blueprint/LeaderLounge/BP_Dynamic_Value Object Reference"))
  (return null))

(fn `OnRep_InteractToggle`
  (if (`self.InteractToggle`)
    _))

(fn `ScoreRef`
  (params (UpdateTrustScore :type Integer) (UpdateValueScore :type Integer))
  (return))

(fn `trustSelectedCountRef`
  (returns (CounterTrust :type "/Game/Blueprint/BP_Counter_Trust Object Reference"))
  (return null))

(fn `UserConstructionScript`)

(fn `valueSelectedCountRef`
  (returns (counterValue :type "/Game/Blueprint/BP_Counter_Value Object Reference"))
  (return null))