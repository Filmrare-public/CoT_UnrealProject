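; Leader-lounge circle graph actor that plots brand coins in a vertical ring at 36-degree steps, one per BP_ranking trust bar.
; BP_DataLayer scores set each coin's radius (trust) and scale (value); the ranking page offsets only the trust lookup.
; Coins are child actors classed by brand name, destroyed and rebuilt when re-added.
; A toggle switches between showing only the selected brand's coin and all coins.
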(event `self.ReceiveBeginPlay`
  (bind _returnvalue (`GameplayStatics.GetActorOfClass` "/Game/Blueprint/BP_DataLayer.BP_DataLayer_C"))
  (bind _datalayerref (message `/Game/Blueprint/Interfaces/BP_Interact_Interface.getDataLayerRef` _returnvalue))
  (set `self.Data Layer Ref` _datalayerref))

(event `addCoins`
  (bind _returnvalue (`self.GetTransform`))
  (bind _data_layer_ref (`self.Data Layer Ref`))
  (bind _data_layer_ref_2 (`self.Data Layer Ref`))
  (if (> (`KismetArrayLibrary.Array_Length` (`self.brandCoinsArray`)) 0)
    (`self.clearBrandCoins`)
    (else
      (bind _returnvalue_2 (`GameplayStatics.GetActorOfClass` "/Game/Blueprint/LeaderLounge/BP_ranking.BP_ranking_C"))
      (bind _rankingref (message `/Game/Blueprint/Interfaces/BP_Interact_Interface.getRankingRef` _returnvalue_2))
      (`|ExecutionSequence`
        (:`then_0`
          (if (`/Game/Blueprint/LeaderLounge/BP_ranking.pageNumber` _rankingref)
            (set `self.arrayOffset` 10)
            (else
              (set `self.arrayOffset` 0))))
        (:`then_1`
          (for (_array_element _array_index) (`/Game/Blueprint/LeaderLounge/BP_ranking.trustBars` _rankingref)
            (`|ExecutionSequence`
              (:`then_0`
                (bind _barref (message `/Game/Blueprint/Interfaces/BP_Interact_Interface.getBarRef` _array_element)))
              (:`then_1`
                (bind _output_get (set `self.radius` (`KismetMathLibrary.MapRangeClamped` (`KismetMathLibrary.Conv_IntToDouble` (`|GetArrayItem` (`/Game/Blueprint/BP_DataLayer.trustScoreArray` _data_layer_ref) (+ (`self.arrayOffset`) _array_index))) (`KismetMathLibrary.Conv_IntToDouble` (`/Game/Blueprint/BP_DataLayer.trustMin` _data_layer_ref)) (`KismetMathLibrary.Conv_IntToDouble` (`/Game/Blueprint/BP_DataLayer.trustMax` _data_layer_ref)) 200.0)))
                (bind _returnvalue_3 (* (/ (`KismetMathLibrary.GetPI`) 180.0) (* _array_index 36)))
                (bind _returnvalue_4 (`AddComponent|NODE_AddChildActorComponent-0` :`bManualAttachment` true :`RelativeTransform` (`KismetMathLibrary.MakeTransform` (`KismetMathLibrary.MakeVector` (+ (.x (.location _returnvalue)) (* (`KismetMathLibrary.Cos` _returnvalue_3) _output_get)) (.y (.location _returnvalue)) (+ (.z (.location _returnvalue)) (* (`KismetMathLibrary.Sin` _returnvalue_3) _output_get))) (struct :`Yaw` 90.0) (`KismetMathLibrary.Conv_DoubleToVector` (`KismetMathLibrary.MapRangeClamped` (`KismetMathLibrary.Conv_IntToDouble` (`|GetArrayItem` (`/Game/Blueprint/BP_DataLayer.valueScoreArray` _data_layer_ref_2) _array_index)) (`KismetMathLibrary.Conv_IntToDouble` (`/Game/Blueprint/BP_DataLayer.valueMax` _data_layer_ref_2)) (`KismetMathLibrary.Conv_IntToDouble` (`/Game/Blueprint/BP_DataLayer.valueMin` _data_layer_ref_2)) 0.6 0.2)))))
                (`ChildActorComponent.SetChildActorClass` _returnvalue_4 (`BlueprintMapLibrary.Map_Find` (`/Game/Blueprint/LeaderLounge/BP_ranking.coinsArray_Test` _rankingref) (`/Game/Blueprint/LeaderLounge/BP_Dynamic_bar.brandName` _barref)))
                (`KismetArrayLibrary.Array_Add` (`self.brandCoinsArray`) (`ChildActorComponent.ChildActor` _returnvalue_4))))))))))

(event `clearBrandCoins`
  (bind _brandcoinsarray (`self.brandCoinsArray`))
  ;[1 1 1] RemoveCoins
  (for _array_element _brandcoinsarray
    (`self.K2_DestroyActor` _array_element))
  (`KismetArrayLibrary.Array_Clear` _brandcoinsarray)
  (`self.addCoins`))

(event `toggleBrandCoins`
  ;[1 1 1] showonlyselectedcoin
  (set `self.selected` (not (`self.selected`)))
  (for _array_element (`self.brandCoinsArray`)
    (bind _getbrandcoinref (message `/Game/Blueprint/brandCoins/BI_brandCoins.getBrandCoinRef` _array_element))
    (if (`self.selected`)
      (bind _rootcomponent (`Actor.RootComponent` _array_element))
      (`SceneComponent.SetVisibility` _rootcomponent (== (`self.selectedBrandName`) (`/Game/Blueprint/brandCoins/BP_BrandCoin.coinName` _getbrandcoinref)) true)
      (else
        (`SceneComponent.SetVisibility` _rootcomponent true true)))))

(fn `getBarRef`
  (returns (barRef :type "/Game/Blueprint/LeaderLounge/BP_Dynamic_bar Object Reference"))
  (return null))

(fn `getBarRefVal`
  (returns (getBarRefVal :type "/Game/Blueprint/LeaderLounge/BP_Dynamic_Value Object Reference"))
  (return null))

(fn `getBijuRef`
  (returns (bijuRef :type "/Game/ThirdPerson/Blueprints/BP_BijuNPC Object Reference"))
  (return null))

(fn `getBrandCoinRef`
  (returns (getBrandCoinRef :type "/Game/Blueprint/brandCoins/BP_BrandCoin Object Reference"))
  (return null))

(fn `getCircleGraphRef`
  (returns (circleGraphRef :type "/Game/Blueprint/LeaderLounge/BP_CircleGraph Object Reference"))
  (return self))

(fn `getDataLayerRef`
  (returns (dataLayerRef :type "/Game/Blueprint/BP_DataLayer Object Reference"))
  (return null))

(fn `getDoorRef`
  (returns (doorRef :type "/Game/Assets/door/BP_Door Object Reference"))
  (return null))

(fn `getHUDRef`
  (returns (hudRef :type "/Game/RPMCharacterTool/HUD/BP_HUD Object Reference"))
  (return null))

(fn `getRankingRef`
  (returns (rankingRef :type "/Game/Blueprint/LeaderLounge/BP_ranking Object Reference"))
  (return null))

(fn `getTopBrandRef`
  (returns (topBrandRef :type "/Game/Blueprint/BP_LeaderOfWeek Object Reference"))
  (return null))

(fn `getValueBarRef`
  (returns (valueBarref :type "/Game/Blueprint/LeaderLounge/BP_Dynamic_Value Object Reference"))
  (return null))

(fn `UserConstructionScript`)