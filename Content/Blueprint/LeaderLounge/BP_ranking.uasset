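; Leader Lounge ranking board actor that shows brand trust and value scores as paired rows of bars with brand coins.
; The construction script spawns both bar columns as child actors.
; UpdateBars fills them from BP_DataLayer, using PageNumber to offset by ten entries, then rebuilds coin actors looked up by brand name and copies coin names to value bars.
; Actors reach each other through reference-getter messages, with GetRankingRef returning this board.
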(event `self.ReceiveBeginPlay`
  (bind _returnvalue (`GameplayStatics.GetActorOfClass` "/Game/Blueprint/BP_DataLayer.BP_DataLayer_C"))
  (bind _datalayerref (message `/Game/Blueprint/Interfaces/BP_Interact_Interface.getDataLayerRef` _returnvalue))
  (set `self.Data Layer Ref` _datalayerref))

(event `updateBars`
  (bind _data_layer_ref (`self.Data Layer Ref`))
  (bind _data_layer_ref_2 (`self.Data Layer Ref`))
  (`|ExecutionSequence`
    (:`then_0`
      (if (`self.pageNumber`)
        (set `self.arrayOffset` 10)
        (else
          (set `self.arrayOffset` 0))))
    (:`then_1`
      (for (_array_element _array_index) (`self.trustBars`)
        (bind _barref (message `/Game/Blueprint/Interfaces/BP_Interact_Interface.getBarRef` _array_element))
        (bind _returnvalue (+ _array_index (`self.arrayOffset`)))
        (set `/Game/Blueprint/LeaderLounge/BP_Dynamic_bar.barValue` (`KismetMathLibrary.Conv_IntToDouble` (`|GetArrayItem` (`/Game/Blueprint/BP_DataLayer.trustScoreArray` _data_layer_ref) _returnvalue)) _barref)
        (set `/Game/Blueprint/LeaderLounge/BP_Dynamic_bar.userInputMinimum` (`KismetMathLibrary.Conv_IntToDouble` (`/Game/Blueprint/BP_DataLayer.trustMin` _data_layer_ref)) _barref)
        (set `/Game/Blueprint/LeaderLounge/BP_Dynamic_bar.userInputMaximum` (`KismetMathLibrary.Conv_IntToDouble` (`/Game/Blueprint/BP_DataLayer.trustMax` _data_layer_ref)) _barref)
        (bind _keys (`BlueprintMapLibrary.Map_Keys` (`/Game/Blueprint/BP_DataLayer.TrustScore` _data_layer_ref)))
        (set `/Game/Blueprint/LeaderLounge/BP_Dynamic_bar.brandName` (`|GetArrayItem` _keys _returnvalue) _barref)
        (`/Game/Blueprint/LeaderLounge/BP_Dynamic_bar.updateValue` _barref))
      (`self.addbrandcoins`))
    (:`then_2`
      (for (_array_element_2 _array_index_2) (`self.valueBars`)
        (bind _valuebarref (message `/Game/Blueprint/Interfaces/BP_Interact_Interface.getValueBarRef` _array_element_2))
        (set `/Game/Blueprint/LeaderLounge/BP_Dynamic_Value.barValue` (`KismetMathLibrary.Conv_IntToDouble` (`|GetArrayItem` (`/Game/Blueprint/BP_DataLayer.valueScoreArray` _data_layer_ref_2) (+ _array_index_2 (`self.arrayOffset`)))) _valuebarref)
        (set `/Game/Blueprint/LeaderLounge/BP_Dynamic_Value.userInputMaximum` (`KismetMathLibrary.Conv_IntToDouble` (`/Game/Blueprint/BP_DataLayer.valueMax` _data_layer_ref_2)) _valuebarref)
        (set `/Game/Blueprint/LeaderLounge/BP_Dynamic_Value.userInputMinimum` (`KismetMathLibrary.Conv_IntToDouble` (`/Game/Blueprint/BP_DataLayer.valueMin` _data_layer_ref_2)) _valuebarref)
        (`/Game/Blueprint/LeaderLounge/BP_Dynamic_Value.updateValue` _valuebarref)))))

(event `addbrandcoins`
  (bind _returnvalue_location (`KismetMathLibrary.BreakTransform` (`self.GetTransform` self)))
  (if (> (`KismetArrayLibrary.Array_Length` (`self.coins`)) 0)
    (`self.clearCoinsArray`)
    (else
      (`|ExecutionSequence`
        (:`then_0`
          (if (`self.pageNumber`)
            (set `self.arrayOffset` 10)
            (else
              (set `self.arrayOffset` 0))))
        (:`then_1`
          (for (_array_element _array_index) (`self.trustBars`)
            (bind _barref (message `/Game/Blueprint/Interfaces/BP_Interact_Interface.getBarRef` _array_element))
            (bind _returnvalue (`AddComponent|NODE_AddChildActorComponent-4` :`bManualAttachment` true :`RelativeTransform` (`KismetMathLibrary.MakeTransform` (`KismetMathLibrary.MakeVector` (- (.x _returnvalue_location) 25.0) (.y _returnvalue_location) (- (.z _returnvalue_location) (* (+ _array_index 1) 40))) (struct :`Yaw` 90.0) (0.3 0.3 0.3))))
            (bind _value (`BlueprintMapLibrary.Map_Find` (`self.coinsArray_Test`) (`/Game/Blueprint/LeaderLounge/BP_Dynamic_bar.brandName` _barref)))
            (`ChildActorComponent.SetChildActorClass` _returnvalue _value)
            (`KismetArrayLibrary.Array_Add` (`self.coins`) (`ChildActorComponent.ChildActor` _returnvalue))
            (bind _returnvalue_2 (`GameplayStatics.GetActorOfClass` _value))
            (bind _getbrandcoinref (message `/Game/Blueprint/brandCoins/BI_brandCoins.getBrandCoinRef` _returnvalue_2))
            (bind _valuebarref (message `/Game/Blueprint/Interfaces/BP_Interact_Interface.getValueBarRef` (`|GetArrayItem` (`self.valueBars`) _array_index)))
            (set `/Game/Blueprint/LeaderLounge/BP_Dynamic_Value.brandName` (`/Game/Blueprint/brandCoins/BP_BrandCoin.coinName` _getbrandcoinref) _valuebarref)))))))

(event `clearCoinsArray`
  (bind _coins (`self.coins`))
  ;[1 1 1] RemoveCoins
  (for _array_element _coins
    (`self.K2_DestroyActor` _array_element))
  (`KismetArrayLibrary.Array_Clear` _coins)
  (`self.addbrandcoins`))

(fn `getBarRef`
  (returns (barRef :type "/Game/Blueprint/LeaderLounge/BP_Dynamic_bar Object Reference"))
  (return null))

(fn `getBarRefVal`
  (returns (getBarRefVal :type "/Game/Blueprint/LeaderLounge/BP_Dynamic_Value Object Reference"))
  (return null))

(fn `getBijuRef`
  (returns (bijuRef :type "/Game/ThirdPerson/Blueprints/BP_BijuNPC Object Reference"))
  (return null))

(fn `getBrandCoinRef`
  (returns (getBrandCoinRef :type "/Game/Blueprint/brandCoins/BP_BrandCoin Object Reference"))
  (return null))

(fn `getCircleGraphRef`
  (returns (circleGraphRef :type "/Game/Blueprint/LeaderLounge/BP_CircleGraph Object Reference"))
  (return null))

(fn `getDataLayerRef`
  (returns (dataLayerRef :type "/Game/Blueprint/BP_DataLayer Object Reference"))
  (return null))

(fn `getDoorRef`
  (returns (doorRef :type "/Game/Assets/door/BP_Door Object Reference"))
  (return null))

(fn `getHUDRef`
  (returns (hudRef :type "/Game/RPMCharacterTool/HUD/BP_HUD Object Reference"))
  (return null))

(fn `getRankingRef`
  (returns (rankingRef :type "/Game/Blueprint/LeaderLounge/BP_ranking Object Reference"))
  (return self))

(fn `getTopBrandRef`
  (returns (topBrandRef :type "/Game/Blueprint/BP_LeaderOfWeek Object Reference"))
  (return null))

(fn `getValueBarRef`
  (returns (valueBarref :type "/Game/Blueprint/LeaderLounge/BP_Dynamic_Value Object Reference"))
  (return null))

(fn `UserConstructionScript`
  (bind _index (`self.index`))
  (bind (_returnvalue_location _returnvalue_rotation _returnvalue_scale) (`KismetMathLibrary.BreakTransform` (`self.GetTransform` self)))
  (bind _x (.x _returnvalue_location))
  (bind _y (.y _returnvalue_location))
  (bind _returnvalue (- (.z _returnvalue_location) (* _index 40.0)))
  (`|ExecutionSequence`
    (:`then_0`
      (`KismetArrayLibrary.Array_Clear` (`self.trustBars`)))
    (:`then_1`
      (`KismetArrayLibrary.Array_Clear` (`self.valueBars`)))
    (:`then_2`
      (while (< _index (`self.length`))
        (`/Engine/EditorBlueprintResources/StandardMacros.IncrementInt` (`self.index`)
          (:`  `
            (`|ExecutionSequence`
              (:`then_0`
                (bind _returnvalue_2 (`AddComponent|NODE_AddChildActorComponent-3` :`bManualAttachment` true :`RelativeTransform` (`KismetMathLibrary.MakeTransform` (`KismetMathLibrary.MakeVector` (+ _x -50.0) _y _returnvalue) _returnvalue_rotation _returnvalue_scale)))
                (`ChildActorComponent.SetChildActorClass` _returnvalue_2 "/Game/Blueprint/LeaderLounge/BP_Dynamic_Value.BP_Dynamic_Value_C")
                (`KismetArrayLibrary.Array_Add` (`self.valueBars`) (`ChildActorComponent.ChildActor` _returnvalue_2)))
              (:`then_1`
                (bind _returnvalue_3 (`AddComponent|NODE_AddChildActorComponent-2` :`bManualAttachment` true :`RelativeTransform` (`KismetMathLibrary.MakeTransform` (`KismetMathLibrary.MakeVector` _x _y _returnvalue) _returnvalue_rotation _returnvalue_scale)))
                (`ChildActorComponent.SetChildActorClass` _returnvalue_3 "/Game/Blueprint/LeaderLounge/BP_Dynamic_bar.BP_Dynamic_bar_C")
                (`KismetArrayLibrary.Array_Add` (`self.trustBars`) (`ChildActorComponent.ChildActor` _returnvalue_3))))))))))