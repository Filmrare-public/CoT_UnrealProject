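; BP_Carousel is a rotating 3D ring of selectable brand orbs, built from ItemsClass as child actors in the construction script.
; NextItem and PreviousItem turn it one slot with timelines, offsetting the selected orb's position and writing the brand to BP_DataLayer.
; RotateToSelectedOrb picks the shorter direction by name index, then chains steps until SelectedBrand matches SelectedOrb.
; The first such selection also notifies BP_BijuNPC.
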(event `self.ReceiveBeginPlay`
  ;[1 1 1] Edit Rotation Speed
  (`TimelineComponent.SetPlayRate` (`self.Timeline_NextItem`) (`self.RotationSpeed`))
  (`TimelineComponent.SetPlayRate` (`self.Timeline_PreviousItem`) (`self.RotationSpeed`))
  ;[1 1 1] Get data from first item
  (bind _returnvalue (`GameplayStatics.GetActorOfClass` "/Game/Blueprint/BP_DataLayer.BP_DataLayer_C"))
  (bind _datalayerref (message `/Game/Blueprint/Interfaces/BP_Interact_Interface.getDataLayerRef` _returnvalue))
  (bind _output_get (set `self.Data Layer Ref` _datalayerref))
  (set `/Game/Blueprint/BP_DataLayer.selectedOrb` "test" _output_get)
  (set `self.fromOrbSelection` true)
  (set `self.resetSelection` false)
  (`self.SelectedItemData` (`|GetArrayItem` (`self.Items`) 3)))

(event `NextItem`
  (bind _selecteditemactor (`self.SelectedItemActor`))
  (bind _returnvalue (/ 360.0 (`KismetMathLibrary.Conv_IntToDouble` (`KismetArrayLibrary.Array_Length` (`self.ItemsClass`)))))
  (bind _returnvalue_2 (* (`self.CurrentStep`) _returnvalue))
  ;[1 1 1] Next Item
  (if (not (`self.IsRotating`))
    (`|ExecutionSequence`
      (:`then_0`
        (if (or (`self.resetSelection`) (not (`self.fromOrbSelection`)))
          (`self.K2_SetActorLocation` _selecteditemactor (`KismetMathLibrary.MakeVector` (.x (`self.K2_GetActorLocation` _selecteditemactor)) (+ (.y (`self.K2_GetActorLocation` _selecteditemactor)) 10.0) (+ (.z (`self.K2_GetActorLocation` _selecteditemactor)) 150.0)) false false)))
      (:`then_1`
        (`/Engine/EditorBlueprintResources/StandardMacros.IncrementInt` (`self.CurrentStep`)
          (:`  `
            (set `self.IsRotating` true)
            (bind (_direction _alpha) (`Timeline|Timeline_NextItem` :!via `PlayFromStart`)
              (:`Update`
                (`self.K2_SetActorRelativeRotation` (`KismetMathLibrary.MakeRotator` 0.0 0.0 (`KismetMathLibrary.Lerp` (- _returnvalue_2 _returnvalue) _returnvalue_2 _alpha))))
              (:`Finished`
                (`|ExecutionSequence`
                  (:`then_0`
                    (if (>= (`self.CurrentStep`) (`KismetArrayLibrary.Array_Length` (`self.Items`)))
                      (set `self.CurrentStep` 0))
                    (set `self.IsRotating` false)
                    (set `self.resetSelection` false)
                    (`self.CurrentSelectedItem` true)))))))))))

(event `CurrentSelectedItem`
  (params (IsNext :type Boolean))
  ;[1 1 1] Obtain the selected item Index
  (if IsNext
    (`/Engine/EditorBlueprintResources/StandardMacros.DecrementInt` (`self.SelectedItem`)
      (:`  `
        (if (< (`self.SelectedItem`) 0)
          (set `self.SelectedItem` (- (`KismetArrayLibrary.Array_Length` (`self.Items`)) 1)))))
    (else
      (`/Engine/EditorBlueprintResources/StandardMacros.IncrementInt` (`self.SelectedItem`)
        (:`  `
          (if (>= (`self.SelectedItem`) (`KismetArrayLibrary.Array_Length` (`self.Items`)))
            (set `self.SelectedItem` 0))))))
  ;;[1 1 1] Retrieve the selected item's data
  (`self.SelectedItemData` (`|GetArrayItem` (`self.Items`) (`self.SelectedItem`))))

(event `SelectedItemData`
  (params (Actor :type "Actor Object Reference"))
  ;[1 1 1] Obtain the selected item Index
  ;;[1 1 1] Retrieve the selected item's data
  (bind _output_get (set `self.SelectedItemActor` Actor))
  (`|ExecutionSequence`
    (:`then_0`
      (if (`self.firstBrandSelected`)
        (bind _orbref (message `/Game/Blueprint/brandBubble/BI_BrandOrbInterface.getOrbRef` _output_get))
        (bind _returnvalue (`GameplayStatics.GetActorOfClass` "/Game/Blueprint/BP_DataLayer.BP_DataLayer_C"))
        (bind _datalayerref (message `/Game/Blueprint/Interfaces/BP_Interact_Interface.getDataLayerRef` _returnvalue))
        (set `/Game/Blueprint/BP_DataLayer.selectedBrand` (`KismetStringLibrary.Conv_NameToString` (`/Game/Blueprint/brandBubble/BP_BrandOrbItem.orbName` _orbref)) _datalayerref)
        (set `self.keepRotating` true)
        (else
          (message `/Game/Blueprint/brandBubble/BI_BrandOrbInterface.getOrbRef` _output_get)
          (bind _returnvalue_2 (`GameplayStatics.GetActorOfClass` "/Game/Blueprint/BP_DataLayer.BP_DataLayer_C"))
          (bind _datalayerref_2 (message `/Game/Blueprint/Interfaces/BP_Interact_Interface.getDataLayerRef` _returnvalue_2))
          (set `/Game/Blueprint/BP_DataLayer.selectedBrand` "facebook" _datalayerref_2))))
    (:`then_1`
      (if (`self.fromOrbSelection`)
        (bind _returnvalue_3 (`GameplayStatics.GetActorOfClass` "/Game/Blueprint/BP_DataLayer.BP_DataLayer_C"))
        (bind _datalayerref_3 (message `/Game/Blueprint/Interfaces/BP_Interact_Interface.getDataLayerRef` _returnvalue_3))
        (if (!= (`/Game/Blueprint/BP_DataLayer.selectedBrand` _datalayerref_3) (`/Game/Blueprint/BP_DataLayer.selectedOrb` _datalayerref_3))
          (if (`self.keepRotating`)
            (if (`self.direction`)
              (`self.PreviousItem`)
              (else
                (`self.NextItem`))))
          (else
            (set `self.fromOrbSelection` false)
            (`self.K2_SetActorLocation` _output_get (`KismetMathLibrary.MakeVector` (.x (`self.K2_GetActorLocation` Actor)) (+ (.y (`self.K2_GetActorLocation` Actor)) -10.0) (+ (.z (`self.K2_GetActorLocation` Actor)) -150.0)) false false :!label _label)))
        (else
          (goto _label))))))

(event `PreviousItem`
  (bind _selecteditemactor (`self.SelectedItemActor`))
  (bind _returnvalue (/ 360.0 (`KismetMathLibrary.Conv_IntToDouble` (`KismetArrayLibrary.Array_Length` (`self.ItemsClass`)))))
  (bind _returnvalue_2 (* (`self.CurrentStep`) _returnvalue))
  ;[1 1 1] Previous Item
  (if (not (`self.IsRotating`))
    (`|ExecutionSequence`
      (:`then_0`
        (if (or (`self.resetSelection`) (not (`self.fromOrbSelection`)))
          (`self.K2_SetActorLocation` _selecteditemactor (`KismetMathLibrary.MakeVector` (.x (`self.K2_GetActorLocation` _selecteditemactor)) (+ (.y (`self.K2_GetActorLocation` _selecteditemactor)) 10.0) (+ (.z (`self.K2_GetActorLocation` _selecteditemactor)) 150.0)) false false)))
      (:`then_1`
        (`/Engine/EditorBlueprintResources/StandardMacros.DecrementInt` (`self.CurrentStep`)
          (:`  `
            (set `self.IsRotating` true)
            (bind (_direction _alpha) (`Timeline|Timeline_PreviousItem` :!via `PlayFromStart`)
              (:`Update`
                (`self.K2_SetActorRelativeRotation` (`KismetMathLibrary.MakeRotator` 0.0 0.0 (`KismetMathLibrary.Lerp` (+ _returnvalue_2 _returnvalue) _returnvalue_2 _alpha))))
              (:`Finished`
                (if (< (`self.CurrentStep`) 0)
                  (set `self.CurrentStep` (- (`KismetArrayLibrary.Array_Length` (`self.Items`)) 1)))
                (set `self.IsRotating` false)
                (set `self.resetSelection` false)
                (`self.CurrentSelectedItem` false)))))))))

(event `RotateToSelectedOrb`
  (bind _data_layer_ref (`self.Data Layer Ref`))
  (bind _orbnames (`self.orbNames`))
  (bind _returnvalue (`KismetArrayLibrary.Array_Find` _orbnames (`/Game/Blueprint/BP_DataLayer.selectedBrand` _data_layer_ref)))
  (bind _returnvalue_2 (`KismetArrayLibrary.Array_Find` _orbnames (`/Game/Blueprint/BP_DataLayer.selectedOrb` _data_layer_ref)))
  (if (`self.firstBrandSelected`)
    (set `self.resetSelection` true)
    (else
      (bind _returnvalue_3 (`GameplayStatics.GetActorOfClass` "/Game/ThirdPerson/Blueprints/BP_BijuNPC.BP_BijuNPC_C"))
      (bind _bijuref (message `/Game/Blueprint/Interfaces/BP_Interact_Interface.getBijuRef` _returnvalue_3))
      (`/Game/ThirdPerson/Blueprints/BP_BijuNPC.brandSelected` _bijuref)
      (set `self.firstBrandSelected` true)
      (set `self.resetSelection` false)))
  (set `self.fromOrbSelection` true)
  (set `self.internal` (< (- (`KismetMathLibrary.Max` _returnvalue _returnvalue_2) (`KismetMathLibrary.Min` _returnvalue _returnvalue_2)) (/ (- (`KismetArrayLibrary.Array_Length` _orbnames) 0) 2)))
  (if (or (and (`self.internal`) (< _returnvalue _returnvalue_2)) (and (> _returnvalue _returnvalue_2) (not (`self.internal`))))
    (set `self.direction` true)
    (`self.PreviousItem`)
    (else
      (set `self.direction` false)
      (`self.NextItem`))))

(fn `getCarouselRef`
  (returns (carouselRef :type "/Game/3DCarousel/Blueprint/BP_Carousel Object Reference"))
  (return self))

(fn `getOrbRef`
  (returns (orbRef :type "/Game/Blueprint/brandBubble/BP_BrandOrbItem Object Reference"))
  (return null))

(fn `UserConstructionScript`
  (bind (_returnvalue_x _returnvalue_y) (`KismetMathLibrary.BreakVector` (`self.K2_GetActorLocation`)))
  (bind _returnvalue (`KismetArrayLibrary.Array_Length` (`self.ItemsClass`)))
  (bind _returnvalue_2 (/ 360.0 (`KismetMathLibrary.Conv_IntToDouble` _returnvalue)))
  (`SceneComponent.K2_SetRelativeLocation` (`self.Arrow`) (`KismetMathLibrary.MakeVector` 300.0 (+ _returnvalue_y (`self.Radius`)) 300.0) false false)
  (for _index (range 1 (+ _returnvalue 1))
    (bind _returnvalue_3 (`KismetMathLibrary.GreaterGreater_VectorRotator` (`KismetMathLibrary.MakeVector` (`self.Radius`)) (`KismetMathLibrary.MakeRotator` 0.0 0.0 (+ (* _index _returnvalue_2) (`KismetMathLibrary.MapRangeClamped` (`self.Offset`) 0.0 1.0 0.0 _returnvalue_2)))))
    (bind _returnvalue_4 (`AddComponent|NODE_AddChildActorComponent-1` :`RelativeTransform` (`KismetMathLibrary.MakeTransform` _returnvalue_3 (`KismetMathLibrary.Conv_VectorToRotator` _returnvalue_3))))
    (`ChildActorComponent.SetChildActorClass` _returnvalue_4 (`|GetArrayItem` (`self.ItemsClass`) (- _index 1)))
    (bind _childactor (`ChildActorComponent.ChildActor` _returnvalue_4))
    (`KismetArrayLibrary.Array_Add` (`self.Items`) _childactor)
    (bind _orbref (message `/Game/Blueprint/brandBubble/BI_BrandOrbInterface.getOrbRef` _childactor))
    (`KismetArrayLibrary.Array_Add` (`self.orbNames`) (`KismetStringLibrary.Conv_NameToString` (`/Game/Blueprint/brandBubble/BP_BrandOrbItem.orbName` _orbref)))))